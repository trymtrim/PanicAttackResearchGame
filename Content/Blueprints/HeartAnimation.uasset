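; Blueprint that animates a heart sprite with a looping breathing-style scale pulse.
; Each Tick, a timer ping-pongs between zero and BreathingInterval by adding or subtracting DeltaSeconds, flipping direction at either end.
; That timer directly drives a Lerp setting HeartSprite's uniform relative scale; the division normalizing it by the interval is left unused, so the interval affects both period and amplitude.
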(event `self.ReceiveTick`
  (params (DeltaSeconds :type "Float (single-precision)"))
  (`|ExecutionSequence`
    (:`then_0`
      (if (>= (`self.CurrentBreathingTime`) (`self.BreathingInterval`))
        (set `self.CountUpwards` false)
        (elif (<= (`self.CurrentBreathingTime`) 0.0)
          (set `self.CountUpwards` true))))
    (:`then_1`
      (if (`self.CountUpwards`)
        (set `self.CurrentBreathingTime` (+ (`self.CurrentBreathingTime`) DeltaSeconds))
        (else
          (set `self.CurrentBreathingTime` (- (`self.CurrentBreathingTime`) DeltaSeconds)))))
    (:`then_2`
      (`SceneComponent.SetRelativeScale3D` (`self.heart_Sprite`) (`KismetMathLibrary.Conv_DoubleToVector` (`KismetMathLibrary.Lerp` 0.85 1.2 (`self.CurrentBreathingTime`)))))))

(fn `UserConstructionScript`)